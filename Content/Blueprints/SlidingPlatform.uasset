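; Sliding platform actor that moves between its starting position and a local-space end offset, converted to world space at BeginPlay.
; Trigger plays a timeline that lerps the location with unswept teleports, and UnTrigger reverses it after playing a 2D rise/fall sound.
; PlatformRiseFall audio runs during timeline updates and stops on finish.
; Custom time dilation is set to 1/Speed, so higher Speed values mean slower travel.
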(event EventBeginPlay
  (Variables|Default|SetStartLocation (Transformation|GetActorLocation))
  (Variables|Default|SetActualEndLocation (Math|Transform|TransformLocation (Transformation|GetActorTransform) (Variables|Default|GetEndLocation)))
  (Variables|Default|SetCustomTimeDilation (/ 1.0 (Variables|Default|GetSpeed))))

(event Collision|EventActorBeginOverlap
  (params (OtherActor :type Actor%20Object%20Reference)))

(event EventTick
  (params (DeltaSeconds :type Float%20%28single-precision%29)))

(event EventTrigger
  (params (It%20was%20me,%20Dio! :type Actor%20Object%20Reference))
  (bind _platform_rise_fall (Variables|Default|GetPlatform_Rise_Fall))
  (bind _newtrack_0 (Timeline|Timeline_0 Play)
    (:Update
      (Transformation|SetActorLocation (Math|Vector|Lerp(Vector) (Variables|Default|GetStartLocation) (Variables|Default|GetActualEndLocation) _newtrack_0) false true)
      (if (not (Audio|Components|Audio|IsPlaying _platform_rise_fall))
        (Audio|Components|Audio|Play _platform_rise_fall 0.0)))
    (:Finished
      (Audio|Components|Audio|Stop (Variables|Default|GetPlatform_Rise_Fall)))))

(event EventUnTrigger
  (params (It%20was%20me,%20Dio! :type Actor%20Object%20Reference))
  (bind _platform_rise_fall (Variables|Default|GetPlatform_Rise_Fall))
  (Audio|PlaySound2D "/Game/Audio/Platform_Rise_Fall.Platform_Rise_Fall")
  (bind _newtrack_0 (Timeline|Timeline_0 Reverse)
    (:Update
      (Transformation|SetActorLocation (Math|Vector|Lerp(Vector) (Variables|Default|GetStartLocation) (Variables|Default|GetActualEndLocation) _newtrack_0) false true)
      (if (not (Audio|Components|Audio|IsPlaying _platform_rise_fall))
        (Audio|Components|Audio|Play _platform_rise_fall 0.0)))
    (:Finished
      (Audio|Components|Audio|Stop (Variables|Default|GetPlatform_Rise_Fall)))))

(fn ConstructionScript)