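; Moving platform actor that travels back and forth continuously between its starting location and a local-space end point.
; On BeginPlay it converts EndLocation to world space and plays a timeline that lerps the position, teleporting without sweep.
; A FlipFlop on the timeline's finish alternates Reverse and Play to keep the loop going.
; Speed comes from setting the actor's CustomTimeDilation from Period instead of changing the timeline's play rate.
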(event EventBeginPlay
  (Variables|Default|SetStartLocation (Transformation|GetActorLocation))
  (Variables|Default|SetActualEndLocation (Math|Transform|TransformLocation (Transformation|GetActorTransform) (Variables|Default|GetEndLocation)))
  (Variables|Default|SetCustomTimeDilation (* (/ 1.0 (Variables|Default|GetPeriod)) 2.0))
  (bind _newtrack_0 (Timeline|Timeline_0 Play)
    (:Update
      (Transformation|SetActorLocation (Math|Vector|Lerp(Vector) (Variables|Default|GetStartLocation) (Variables|Default|GetActualEndLocation) _newtrack_0) false true))
    (:Finished
      (Utilities|FlowControl|FlipFlop
        (:A
          (Timeline|Timeline_0 Reverse))
        (:B
          (Timeline|Timeline_0 Play))))))

(event Collision|EventActorBeginOverlap
  (params (OtherActor :type Actor%20Object%20Reference)))

(event EventTick
  (params (DeltaSeconds :type Float%20%28single-precision%29)))

(fn ConstructionScript)