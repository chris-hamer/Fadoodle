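; KeyHole is a bobbing keyhole actor that accepts the ThirdPersonCharacter's held object and triggers linked actors.
; When the character overlaps the box with a visible held object, it hides that object, sends TriggerMessage to each Theguy entry, hides its own mesh and plays a sound.
; A ping-ponging timeline drives a cosine-eased vertical bob, with a random starting phase and speed set through CustomTimeDilation from Period.
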(event OnComponentBeginOverlap(Box)
  (params (OverlappedComponent :type Primitive%20Component%20Object%20Reference) (OtherActor :type Actor%20Object%20Reference) (OtherComp :type Primitive%20Component%20Object%20Reference) (OtherBodyIndex :type Integer) (bFromSweep :type Boolean) (SweepResult :type Hit%20Result%20Structure%20%28by%20ref%29))
  (bind _asthird_person_character (Utilities|Casting|CastToThirdPersonCharacter OtherActor))
  (if (Rendering|IsVisible (Variables|/Game/ThirdPersonBP/Blueprints/ThirdPersonCharacter.ThirdPersonCharacter_C|GetHeldObject _asthird_person_character))
    (Rendering|SetVisibility (Variables|/Game/ThirdPersonBP/Blueprints/ThirdPersonCharacter.ThirdPersonCharacter_C|GetHeldObject _asthird_person_character) false false)
    (for _array_element (Variables|Default|Gettheguy)
      (Class|Triggerable|Trigger(Message) _array_element self))
    (Rendering|SetVisibility (Variables|Debug|GetStaticMeshComponent) false false)
    (Audio|PlaySound2D "/Game/Audio/Key_In_Keyhole.Key_In_Keyhole")))

(event EventBeginPlay
  (bind _output_get (Variables|Default|SetStartLocation (Transformation|GetActorLocation)))
  (Variables|Default|SetActualEndLocation (+ _output_get "0, 0,5.000000"))
  (Variables|Default|SetCustomTimeDilation (* (/ 1.0 (Variables|Default|GetPeriod)) 2.0))
  (bind _output_get_2 (Variables|Default|Setr (Math|Random|RandomFloat)))
  (Utilities|FlowControl|Sequence
    (:then_0
      (bind _newtrack_0 (Timeline|Timeline_0 SetNewTime)
        (:Update
          (Transformation|SetActorLocation (Math|Vector|Lerp(Vector) (Variables|Default|GetStartLocation) (Variables|Default|GetActualEndLocation) (/ (+ (Math|Trig|Cos(Degrees) (* _newtrack_0 3.6e+02)) 1.0) 2.0)) false true))
        (:Finished
          (Variables|Default|Setr 0.0)
          (Utilities|FlowControl|FlipFlop
            (:A
              (Timeline|Timeline_0 Reverse))
            (:B
              (Timeline|Timeline_0 Play))))))
    (:then_1
      (Timeline|Timeline_0 Play))))

(event Collision|EventActorBeginOverlap
  (params (OtherActor :type Actor%20Object%20Reference)))

(event EventTick
  (params (DeltaSeconds :type Float%20%28single-precision%29)))

(fn ConstructionScript)