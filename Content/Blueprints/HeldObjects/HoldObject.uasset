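; Pickup actor that, when a ThirdPersonCharacter overlaps it, reveals that character's HeldObject component and destroys itself.
; Tick spins the static mesh at a constant roll rate.
; A ping-ponging timeline bobs the actor slightly above its start location along a cosine curve, from a random starting time.
; BeginPlay derives the actor's custom time dilation from Period to set its animation speed.
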(event EventBeginPlay
  (bind _output_get (Variables|Default|SetStartLocation (Transformation|GetActorLocation)))
  (Variables|Default|SetActualEndLocation (+ _output_get "0, 0,5.000000"))
  (Variables|Default|SetCustomTimeDilation (* (/ 1.0 (Variables|Default|GetPeriod)) 2.0))
  (bind _output_get_2 (Variables|Default|Setr (Math|Random|RandomFloat)))
  (Utilities|FlowControl|Sequence
    (:then_0
      (bind _newtrack_0 (Timeline|Timeline_0 SetNewTime)
        (:Update
          (Transformation|SetActorLocation (Math|Vector|Lerp(Vector) (Variables|Default|GetStartLocation) (Variables|Default|GetActualEndLocation) (/ (+ (Math|Trig|Cos(Degrees) (* _newtrack_0 3.6e+02)) 1.0) 2.0)) false true))
        (:Finished
          (Variables|Default|Setr 0.0)
          (Utilities|FlowControl|FlipFlop
            (:A
              (Timeline|Timeline_0 Reverse))
            (:B
              (Timeline|Timeline_0 Play))))))
    (:then_1
      (Timeline|Timeline_0 Play))))

(event Collision|EventActorBeginOverlap
  (params (OtherActor :type Actor%20Object%20Reference))
  (bind _asthird_person_character (Utilities|Casting|CastToThirdPersonCharacter OtherActor))
  (Rendering|SetVisibility (Variables|/Game/ThirdPersonBP/Blueprints/ThirdPersonCharacter.ThirdPersonCharacter_C|GetHeldObject _asthird_person_character) true false)
  (Actor|DestroyActor))

(event EventTick
  (params (DeltaSeconds :type Float%20%28single-precision%29))
  (Transformation|AddLocalRotation (Variables|Default|GetStaticMesh) (Math|Rotator|MakeRotator (* DeltaSeconds 1.2e+02) 0.0 0.0) false false))

(fn ConstructionScript)