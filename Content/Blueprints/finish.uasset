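; Level finish actor for two players that requires each player type to reach its own mesh before loading the next level.
; Overlap events on the two static meshes check the character's PlayerType, set a per-player flag and store the character reference.
; Tick polls both flags and, once only, shows a widget, waits briefly, opens "02_level", then removes the second player and destroys its pawn.
; Flags never reset, so simultaneous overlap is not required.
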(event OnComponentBeginOverlap(StaticMesh)
  (params (OverlappedComponent :type Primitive%20Component%20Object%20Reference) (OtherActor :type Actor%20Object%20Reference) (OtherComp :type Primitive%20Component%20Object%20Reference) (OtherBodyIndex :type Integer) (bFromSweep :type Boolean) (SweepResult :type Hit%20Result%20Structure%20%28by%20ref%29))
  (bind _asthird_person_character (Utilities|Casting|CastToThirdPersonCharacter OtherActor))
  (if (Utilities|Enum|Equal(Enum) (Variables|/Game/ThirdPersonBP/Blueprints/ThirdPersonCharacter.ThirdPersonCharacter_C|GetPlayerType _asthird_person_character) "NewEnumerator0")
    (Variables|Default|Set1 true)
    (Variables|Default|Sets _asthird_person_character)))

(event OnComponentBeginOverlap(StaticMesh1)
  (params (OverlappedComponent :type Primitive%20Component%20Object%20Reference) (OtherActor :type Actor%20Object%20Reference) (OtherComp :type Primitive%20Component%20Object%20Reference) (OtherBodyIndex :type Integer) (bFromSweep :type Boolean) (SweepResult :type Hit%20Result%20Structure%20%28by%20ref%29))
  (bind _asthird_person_character (Utilities|Casting|CastToThirdPersonCharacter OtherActor))
  (if (Utilities|Enum|Equal(Enum) (Variables|/Game/ThirdPersonBP/Blueprints/ThirdPersonCharacter.ThirdPersonCharacter_C|GetPlayerType _asthird_person_character) "NewEnumerator1")
    (Variables|Default|Set2 true)
    (Variables|Default|Setl _asthird_person_character)))

(event EventBeginPlay)

(event Collision|EventActorBeginOverlap
  (params (OtherActor :type Actor%20Object%20Reference)))

(event EventTick
  (params (DeltaSeconds :type Float%20%28single-precision%29))
  (if (and (Variables|Default|Get1) (Variables|Default|Get2))
    (Utilities|FlowControl|DoOnce false
      (:Completed
        (bind _returnvalue (UserInterface|CreateWidget "/Game/NewWidgetBlueprint.NewWidgetBlueprint_C"))
        (UserInterface|Viewport|AddtoViewport _returnvalue 0)
        (Utilities|FlowControl|Delay 4.0)
        (Game|OpenLevel(byName) "02_level")
        (bind _asfadoodle_player_controller (Utilities|Casting|CastToFadoodlePlayerController (Pawn|GetController (Variables|Default|Getl))))
        (Class|GameplayStatics|RemovePlayer _asfadoodle_player_controller true)))))

(fn ConstructionScript)