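; Player controller that lets two local players swap the pawns they control.
; Tab or the gamepad top face button calls Switch, which gets the pawns of player controllers 0 and 1 and has each controller possess the other's pawn.
; An alternative FlipFlop branch inside Switch is disconnected and never runs.
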(event EventBeginPlay)

(event EventTick
  (params (DeltaSeconds :type Float%20%28single-precision%29)))

(event Input|KeyboardEvents|Tab
  (params (Key :type Key%20Structure))
  (:Pressed
    (CallFunction|Switch)))

(event Input|GamepadEvents|GamepadFaceButtonTop
  (params (Key :type Key%20Structure))
  (:Pressed
    (CallFunction|Switch)))

(fn ConstructionScript)

(fn Switch
  (LocalVariables|Set1 (Pawn|GetControlledPawn (Game|GetPlayerController 0)))
  (LocalVariables|Set2 (Pawn|GetControlledPawn (Game|GetPlayerController 1)))
  (Pawn|Possess (Game|GetPlayerController 0) (LocalVariables|Get2))
  (Pawn|Possess (Game|GetPlayerController 1) (LocalVariables|Get1)))