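; PressurePlane is an overlap trigger that activates linked actors when a qualifying character or cube enters it.
; Begin and end overlap both feed Decide, which filters by its Type: any third-person character, one of two player types, or a SpawnedCube.
; Qualifying overlaps send Trigger or UnTrigger messages through the Triggerable interface to each entry in ThingsToTrigger, with DontUntrigger suppressing release.
; An older TargetSize-based check remains as unreachable logic.
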(event EventBeginPlay)

(event Collision|EventActorBeginOverlap
  (params (OtherActor :type Actor%20Object%20Reference))
  (CallFunction|Decide OtherActor false))

(event EventTick
  (params (DeltaSeconds :type Float%20%28single-precision%29)))

(event Collision|EventActorEndOverlap
  (params (OtherActor :type Actor%20Object%20Reference))
  (CallFunction|Decide OtherActor true))

(fn ConstructionScript)

(fn Decide
  (params (Object :type Object%20Object%20Reference) (IsLeaving :type Boolean))
  (bind _asthird_person_character (Utilities|Casting|CastToThirdPersonCharacter Object)
    (:then
      (switch Utilities|FlowControl|Switch|SwitchonESwitchType (Variables|Default|GetType)
        (:NewEnumerator0
          (for _array_element (Variables|Default|GetThingsToTrigger) :!label _label
            (if (Utilities|DoesObjectImplementInterface _array_element "/Game/Blueprints/Triggerable.Triggerable_C")
              (if IsLeaving
                (if (not (Variables|Default|GetDon'tUntrigger))
                  (Class|Triggerable|UnTrigger(Message) _array_element self))
                (else
                  (Class|Triggerable|Trigger(Message) _array_element self))))))
        (:NewEnumerator1
          (if (Utilities|Enum|Equal(Enum) (Variables|/Game/ThirdPersonBP/Blueprints/ThirdPersonCharacter.ThirdPersonCharacter_C|GetPlayerType _asthird_person_character) "NewEnumerator0")
            (goto _label)))
        (:NewEnumerator2
          (if (Utilities|Enum|Equal(Enum) (Variables|/Game/ThirdPersonBP/Blueprints/ThirdPersonCharacter.ThirdPersonCharacter_C|GetPlayerType _asthird_person_character) "NewEnumerator1")
            (goto _label)))))
    (:CastFailed
      (switch Utilities|FlowControl|Switch|SwitchonESwitchType (Variables|Default|GetType)
        (:NewEnumerator4
          (Utilities|Casting|CastToSpawnedCube Object)
          (goto _label))))))