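; ShrinkPanel is a floating pad that sets an overlapping ThirdPersonCharacter's target size to normal, small or large, according to its Type.
; It affects only one player type and triggers the character's grow or shrink animation when the target changes.
; The construction script colors the cube by Type.
; A ping-ponging timeline with random start time drives a cosine vertical bob, its speed set through CustomTimeDilation from Period.
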(event EventBeginPlay
  (bind _output_get (Variables|Default|SetStartLocation (Transformation|GetActorLocation)))
  (Variables|Default|SetActualEndLocation (+ _output_get "0, 0,5.000000"))
  (Variables|Default|SetCustomTimeDilation (* (/ 1.0 (Variables|Default|GetPeriod)) 2.0))
  (bind _output_get_2 (Variables|Default|Setr (Math|Random|RandomFloat)))
  (Utilities|FlowControl|Sequence
    (:then_0
      (bind _newtrack_0 (Timeline|Timeline_0 SetNewTime)
        (:Update
          (Transformation|SetActorLocation (Math|Vector|Lerp(Vector) (Variables|Default|GetStartLocation) (Variables|Default|GetActualEndLocation) (/ (+ (Math|Trig|Cos(Degrees) (* _newtrack_0 3.6e+02)) 1.0) 2.0)) false true))
        (:Finished
          (Variables|Default|Setr 0.0)
          (Utilities|FlowControl|FlipFlop
            (:A
              (Timeline|Timeline_0 Reverse))
            (:B
              (Timeline|Timeline_0 Play))))))
    (:then_1
      (Timeline|Timeline_0 Play))))

(event Collision|EventActorBeginOverlap
  (params (OtherActor :type Actor%20Object%20Reference))
  (bind _asthird_person_character (Utilities|Casting|CastToThirdPersonCharacter OtherActor))
  (if (Utilities|Enum|Equal(Enum) (Variables|/Game/ThirdPersonBP/Blueprints/ThirdPersonCharacter.ThirdPersonCharacter_C|GetPlayerType _asthird_person_character) "NewEnumerator0")
    (Utilities|FlowControl|Sequence
      (:then_0
        (Variables|Default|Setoldtargetsize (Variables|/Game/ThirdPersonBP/Blueprints/ThirdPersonCharacter.ThirdPersonCharacter_C|GetTargetSize _asthird_person_character))
        (switch Utilities|FlowControl|Switch|SwitchonEShrinkType (Variables|Default|GetType)
          (:NewEnumerator0
            (Variables|/Game/ThirdPersonBP/Blueprints/ThirdPersonCharacter.ThirdPersonCharacter_C|SetTargetSize _asthird_person_character 1.0))
          (:NewEnumerator1
            (Variables|/Game/ThirdPersonBP/Blueprints/ThirdPersonCharacter.ThirdPersonCharacter_C|SetTargetSize _asthird_person_character 0.25))
          (:NewEnumerator2
            (Variables|/Game/ThirdPersonBP/Blueprints/ThirdPersonCharacter.ThirdPersonCharacter_C|SetTargetSize _asthird_person_character 2.0))))
      (:then_1
        (if (> (Variables|/Game/ThirdPersonBP/Blueprints/ThirdPersonCharacter.ThirdPersonCharacter_C|GetTargetSize _asthird_person_character) (Variables|Default|Getoldtargetsize))
          (Default|GrowAnimStart _asthird_person_character)
          (elif (< (Variables|/Game/ThirdPersonBP/Blueprints/ThirdPersonCharacter.ThirdPersonCharacter_C|GetTargetSize _asthird_person_character) (Variables|Default|Getoldtargetsize))
            (Default|ShrinkAnimStart _asthird_person_character)))))))

(event EventTick
  (params (DeltaSeconds :type Float%20%28single-precision%29)))

(fn ConstructionScript
  (Rendering|Material|SetMaterial (Variables|Default|GetCube) 0 (Utilities|Select :Index (Variables|Default|GetType) :NewEnumerator0 "/Game/Blueprints/Purple.Purple" :NewEnumerator1 "/Game/Blueprints/Blue.Blue" :NewEnumerator2 "/Game/Blueprints/Red.Red")))